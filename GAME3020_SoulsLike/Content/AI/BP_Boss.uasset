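; Boss enemy that starts its encounter when the player enters its trigger and rewards its defeat with a key.
; The trigger overlap swaps the player's music and creates a named health bar widget bound to the BPCStats component.
; Death shows an "Ancient Enemy Felled" widget and spawns BP_OphulusKey before calling parent death logic; destruction removes the health bar.
; Sword trace start and end positions refresh every tick from world locations.
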(event OnComponentBeginOverlap(BossTrigger)
  (params (OverlappedComponent :type Primitive%20Component%20Object%20Reference) (OtherActor :type Actor%20Object%20Reference) (OtherComp :type Primitive%20Component%20Object%20Reference) (OtherBodyIndex :type Integer) (bFromSweep :type Boolean) (SweepResult :type Hit%20Result%20Structure%20%28by%20ref%29))
  (bind _asbp_third_person_character (Utilities|Casting|CastToBP_ThirdPersonCharacter OtherActor))
  (bind _output_get (Variables|Default|SetPlayerCharacter _asbp_third_person_character))
  (Audio|Components|Audio|SetSound (Variables|/Game/ThirdPerson/Blueprints/BP_ThirdPersonCharacter.BP_ThirdPersonCharacter_C|GetMusicPlayer _output_get) "/Game/SFX/SC_ScarFace.SC_ScarFace")
  (bind _returnvalue (UserInterface|CreateWidget "/Game/UI/HUD/WB_BossHealth.WB_BossHealth_C"))
  (bind _output_get_2 (Variables|Default|SetBossHealthWidget _returnvalue))
  (UserInterface|Viewport|AddtoViewport _output_get_2 0)
  (Utilities|FlowControl|DelayUntilNextTick)
  (Default|SetHealthBar (Variables|Default|GetBPC_Stats) (Variables|/Game/UI/HUD/WB_BossHealth.WB_BossHealth_C|GetHealthBar (Variables|Default|GetBossHealthWidget)))
  (Variables|/Script/UMG.TextBlock|SetText (Variables|/Game/UI/HUD/WB_BossHealth.WB_BossHealth_C|GetBossName (Variables|Default|GetBossHealthWidget)) (Utilities|Text|ToText(String) (Variables|Default|GetName))))

(event EventBeginPlay
  (bind _bpc_stats (Variables|Default|GetBPC_Stats))
  (|CallParentFunction)
  (Variables|Default|SetbossStartSwordTracePos (Transformation|GetWorldLocation (Variables|Default|GetBoss%20Start%20Sword%20Trace%20Pos)))
  (Variables|Default|SetbossEndSwordTracePos (Transformation|GetWorldLocation (Variables|Default|GetBoss%20End%20Sword%20Trace%20Pos)))
  (Variables|/Game/Blueprints/BPC_Stats.BPC_Stats_C|SetHealth _bpc_stats (Variables|/Game/Blueprints/BPC_Stats.BPC_Stats_C|GetMaxHealth _bpc_stats)))

(event Collision|EventActorBeginOverlap
  (params (OtherActor :type Actor%20Object%20Reference)))

(event EventTick
  (params (DeltaSeconds :type Float%20%28single-precision%29))
  (Variables|Default|SetbossStartSwordTracePos (Transformation|GetWorldLocation (Variables|Default|GetBoss%20Start%20Sword%20Trace%20Pos)))
  (Variables|Default|SetbossEndSwordTracePos (Transformation|GetWorldLocation (Variables|Default|GetBoss%20End%20Sword%20Trace%20Pos))))

(event EventDestroyed
  (Widget|RemovefromParent (Variables|Default|GetBossHealthWidget)))

(event EventDie
  (bind _returnvalue (UserInterface|CreateWidget "/Game/UI/GameElements/WB_AncientEnemyFelled.WB_AncientEnemyFelled_C"))
  (UserInterface|Viewport|AddtoViewport _returnvalue 0)
  (Game|SpawnActorfromClass "/Game/Blueprints/Pickups/BP_OphulusKey.BP_OphulusKey_C" (Transformation|GetActorTransform) "Undefined" "MultiplyWithRoot" 0 0)
  (|CallParentFunction))

(fn ConstructionScript
  (|CallParentFunction))