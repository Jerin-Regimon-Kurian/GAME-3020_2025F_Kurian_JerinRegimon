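; BPC_Stats is an actor component that tracks its owner's Health and Stamina and drives their progress bars.
; IncreaseValue adds to the chosen stat, clamps it between zero and its maximum, then updates the assigned bar, validity-checking only the stamina one.
; A looping timer, rather than Tick, regenerates stamina while RegainStamina is true.
; When a health change leaves Health at zero, Die sends DieMessage to the owner.
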(event Custom|Die
  (Class|BPIDamage|Die(Message) (Components|GetOwner)))

(event Custom|SetHealthBar
  (params (HealthBar :type Progress%20Bar%20Object%20Reference))
  (Variables|Default|SetHealth%20Bar HealthBar))

(event Custom|SetStaminaBar
  (params (StaminaBar :type Progress%20Bar%20Object%20Reference))
  (Variables|Default|SetStaminaBar StaminaBar))

(event Custom|RegainStamina
  (if (Variables|Default|GetRegainStamina?)
    (CallFunction|IncreaseValue "NewEnumerator1" 0.1)))

(event EventBeginPlay
  (Utilities|Time|SetTimerbyEvent (delegate Custom|RegainStamina) 0.01 true))

(event EventTick
  (params (DeltaSeconds :type Float%20%28single-precision%29)))

(fn IncreaseValue
  (params (Stat :type E_Stats%20Enum :default "NewEnumerator0") (Value :type Float%20%28double-precision%29))
  (switch Utilities|FlowControl|Switch|SwitchonE_Stats Stat
    (:NewEnumerator0
      (Variables|Default|SetHealth (Math|Float|Clamp(Float) (+ (Variables|Default|GetHealth) Value) 0.0 (Variables|Default|GetMaxHealth)))
      (Utilities|FlowControl|Sequence
        (:then_0
          (if (<= (Variables|Default|GetHealth) 0.0)
            (CallFunction|Die)))
        (:then_1
          (Progress|SetPercent (Variables|Default|GetHealth%20Bar) (/ (Variables|Default|GetHealth) (Variables|Default|GetMaxHealth))))))
    (:NewEnumerator1
      (Variables|Default|SetStamina (Math|Float|Clamp(Float) (+ (Variables|Default|GetStamina) Value) 0.0 (Variables|Default|GetMaxStamina)))
      (bind _staminabar (Variables|Default|GetStaminaBar)
        (:then
          (Progress|SetPercent _staminabar (/ (Variables|Default|GetStamina) (Variables|Default|GetMaxStamina))))
        (:else)))))