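; Buff potion pickup that adds one buff potion to the player when collected.
; On sphere overlap, it casts to BP_ThirdPersonCharacter and increments BuffPotionsLeft on the character's combat component.
; It then writes the new count directly into the HUD inventory slot text, plays a sound at the world origin and destroys itself.
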(event OnComponentBeginOverlap(Sphere)
  (params (OverlappedComponent :type Primitive%20Component%20Object%20Reference) (OtherActor :type Actor%20Object%20Reference) (OtherComp :type Primitive%20Component%20Object%20Reference) (OtherBodyIndex :type Integer) (bFromSweep :type Boolean) (SweepResult :type Hit%20Result%20Structure%20%28by%20ref%29))
  (bind _asbp_third_person_character (Utilities|Casting|CastToBP_ThirdPersonCharacter OtherActor))
  (bind _output_get (Variables|/Game/Blueprints/BPC_Combat.BPC_Combat_C|SetBuffPotionsLeft (Variables|/Game/ThirdPerson/Blueprints/BP_ThirdPersonCharacter.BP_ThirdPersonCharacter_C|GetBPC_Combat _asbp_third_person_character) (+ (Variables|/Game/Blueprints/BPC_Combat.BPC_Combat_C|GetBuffPotionsLeft (Variables|/Game/ThirdPerson/Blueprints/BP_ThirdPersonCharacter.BP_ThirdPersonCharacter_C|GetBPC_Combat _asbp_third_person_character)) 1)))
  (Rendering|Components|TextRender|SetText (Variables|/Game/UI/WB_InventorySlots.WB_InventorySlots_C|GetBuffPotionCount (Variables|/Game/UI/WB_HUD.WB_HUD_C|GetWB_InventorySlots (Variables|/Game/ThirdPerson/Blueprints/BP_ThirdPersonCharacter.BP_ThirdPersonCharacter_C|GetHUD%20Widget _asbp_third_person_character))) (Utilities|Text|ToText(Integer) _output_get))
  (Audio|PlaySoundatLocation 0 "0, 0, 0" "0, 0, 0" 1.0 1.0 0.0 0 0 0 0)
  (Actor|DestroyActor))

(event EventBeginPlay)

(event Collision|EventActorBeginOverlap
  (params (OtherActor :type Actor%20Object%20Reference)))

(event EventTick
  (params (DeltaSeconds :type Float%20%28single-precision%29)))

(fn ConstructionScript)